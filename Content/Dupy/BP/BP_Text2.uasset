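; BP_Text2 is a trigger volume that shows the WBP_secuestrador widget while the top-down character is inside its box.
; On overlap begin it plays the Fade level sequence through a newly created player, then creates the widget, stores it and adds it to the viewport.
; On overlap end it removes the stored widget from its parent.
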(event `self.Box.OnComponentBeginOverlap`
  (params (OverlappedComponent :type "PrimitiveComponent Object Reference") (OtherActor :type "Actor Object Reference") (OtherComp :type "PrimitiveComponent Object Reference") (OtherBodyIndex :type Integer) (bFromSweep :type Boolean) (SweepResult :type "HitResult Structure (by ref)"))
  (cast `/Game/Character/Sprites/BP_TopDownChar` OtherActor)
  (bind _outactor (`LevelSequencePlayer.CreateLevelSequencePlayer` "/Game/Dupy/fade.fade"))
  (`MovieSceneSequencePlayer.Play` (`LevelSequenceActor.SequencePlayer` _outactor))
  (bind _returnvalue (`|CreateWidget` "/Game/Dupy/widget/WBP_secuestrador.WBP_secuestrador_C" (`GameplayStatics.GetPlayerController` 0)))
  (bind _output_get (set `self.s` _returnvalue))
  (`UserWidget.AddToViewport` _output_get 0))

(event `self.Box.OnComponentEndOverlap`
  (params (OverlappedComponent :type "PrimitiveComponent Object Reference") (OtherActor :type "Actor Object Reference") (OtherComp :type "PrimitiveComponent Object Reference") (OtherBodyIndex :type Integer))
  (cast `/Game/Character/Sprites/BP_TopDownChar` OtherActor)
  (`Widget.RemoveFromParent` (`self.s`)))

(fn `UserConstructionScript`)