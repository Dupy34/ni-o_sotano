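; Rotating picture frame puzzle Blueprint that completes when the frame has been turned to its answer position.
; Each interaction plays a timeline that pitches the picture another 90 degrees, ignoring input while it moves.
; When the turn ends, it stores the new rotation and increments a step counter that never wraps.
; A counter matching the answer locks the puzzle, plays an unlock sound and fires the puzzle-completed event.
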(event `self.ReceiveBeginPlay`
  (set `self.StartingRotationFrame` (`SceneComponent.RelativeRotation` (`self.Picture`))))

(event `/Game/Aster(Diego)/Interfaces/BPI_Interaction.Interaction`
  (if (not (`self.Finalized`))
    (`self.RotatingFrame`)))

(event `RotatingFrame`
  (bind (_startingrotationframe_roll _startingrotationframe_pitch) (`KismetMathLibrary.BreakRotator` (`self.StartingRotationFrame`)))
  (bind _frameposition (`self.FramePosition`))
  (if (not (`self.FrameMoving`))
    (set `self.FrameMoving` true)
    (bind (_direction _rotation) (`Timeline|PaintingRotation` :!via `PlayFromStart`)
      (:`Update`
        (bind _returnvalue (`KismetMathLibrary.Lerp` _startingrotationframe_pitch (- _startingrotationframe_pitch 90.0) _rotation))
        (`SceneComponent.K2_SetRelativeRotation` (`self.Picture`) (`KismetMathLibrary.MakeRotator` 0.0 _returnvalue) false false))
      (:`Finished`
        (set `self.StartingRotationFrame` (`KismetMathLibrary.MakeRotator` 0.0 _returnvalue))
        (set `self.FrameMoving` false)
        (bind _result (`/Engine/EditorBlueprintResources/StandardMacros.IncrementInt` _frameposition)
          (:`  `
            (set `self.FramePosition` _result)
            (if (== (`self.PuzzleAnswer`) _frameposition)
              (set `self.Finalized` true)
              (`GameplayStatics.PlaySound2D` "/Game/Aster(Diego)/Sounds/unlock.unlock" 1.0 1.0 0.0 null null)
              (`KismetSystemLibrary.PrintString` "Puzzle finished" true true (struct :`G` 1.0 :`B` 0.026676 :`A` 1.0))
              (`self.EVD_PuzzleCompleted`))))))))

(fn `UserConstructionScript`
  (`parent.UserConstructionScript`))