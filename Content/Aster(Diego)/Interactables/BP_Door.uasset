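; Keypad-locked exit door that opens the Ganaste level when the player character (BP_TopDownChar) overlaps its box while it is open.
; While closed, overlap shows WBP_Keypad with mouse input if CanInteract, otherwise clears widgets and restores game-only input; leaving removes the keypad.
; OpenDoor plays a timeline whose update sets the mesh to a fixed open position and rotation, without interpolation, and flags Open.
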(event `OpenDoor`
  (`Timeline|DoorOpen`
    (:`Update`
      (`SceneComponent.K2_SetRelativeLocation` (`self.StaticMesh`) (-54.0 -49.0 0.0) false false)
      (`SceneComponent.K2_SetRelativeRotation` (`self.StaticMesh`) (`KismetMathLibrary.MakeRotator` 0.0 0.0 90.0) false false)
      (set `self.open?` true))))

(event `self.Box.OnComponentBeginOverlap`
  (params (OverlappedComponent :type "PrimitiveComponent Object Reference") (OtherActor :type "Actor Object Reference") (OtherComp :type "PrimitiveComponent Object Reference") (OtherBodyIndex :type Integer) (bFromSweep :type Boolean) (SweepResult :type "HitResult Structure (by ref)"))
  (bind _returnvalue (`GameplayStatics.GetPlayerController` 0))
  (cast `/Game/Character/Sprites/BP_TopDownChar` OtherActor)
  (if (`self.open?`)
    (`GameplayStatics.OpenLevelBySoftObjectPtr` "/Game/Menu/ganaste.ganaste")
    (elif (`self.CanInteract`)
      (bind _returnvalue_2 (`|CreateWidget` "/Game/Aster(Diego)/UI/WBP_Keypad.WBP_Keypad_C"))
      (`UserWidget.AddToViewport` _returnvalue_2 0)
      (`WidgetBlueprintLibrary.SetInputMode_GameAndUIEx` _returnvalue _returnvalue_2)
      (set `PlayerController.bShowMouseCursor` true _returnvalue)
      (else
        (`WidgetLayoutLibrary.RemoveAllWidgets`)
        (`WidgetBlueprintLibrary.SetInputMode_GameOnly` _returnvalue)
        (set `PlayerController.bShowMouseCursor` false _returnvalue)))))

(event `self.Box.OnComponentEndOverlap`
  (params (OverlappedComponent :type "PrimitiveComponent Object Reference") (OtherActor :type "Actor Object Reference") (OtherComp :type "PrimitiveComponent Object Reference") (OtherBodyIndex :type Integer))
  (cast `/Game/Character/Sprites/BP_TopDownChar` OtherActor)
  (`Widget.RemoveFromParent` (stale `self.Box.OnComponentBeginOverlap` _returnvalue_2)))

(fn `UserConstructionScript`
  (`parent.UserConstructionScript`))