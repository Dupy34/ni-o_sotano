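; BP_Note is an interactable note that shows and hides an on-screen WBP_Codigo widget.
; Each Interaction event flips the IsInteracted flag to toggle the widget between visible and hidden.
; The widget is created and added to the viewport on first use, then cached and reused through visibility changes.
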(event `/Game/Aster(Diego)/Interfaces/BPI_Interaction.Interaction`
  (bind _newvar1 (`self.NewVar1`))
  (bind _output_get (set `self.isInteracted` (not (`self.isInteracted`))))
  (if _output_get
    (`/Engine/EditorBlueprintResources/StandardMacros.IsValid` _newvar1
      (:`Is Valid`
        _)
      (:`Is Not Valid`
        (bind _returnvalue (`|CreateWidget` "/Game/Aster(Diego)/UI/WBP_Codigo.WBP_Codigo_C"))
        (bind _output_get_2 (set `self.NewVar1` _returnvalue))
        (`UserWidget.AddToViewport` _output_get_2 0)))
    (`Widget.SetVisibility` _output_get_2 "Visible")
    (else
      (`/Engine/EditorBlueprintResources/StandardMacros.IsValid` _newvar1
        (:`Is Valid`
          (`Widget.SetVisibility` _output_get_2 "Hidden"))))))

(fn `UserConstructionScript`
  (`parent.UserConstructionScript`))