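; BP_PuzzleGate is a puzzle gate that opens once enough items are collected, then serves as a level exit.
; CollectItem counts pickups and, at the maximum, sets the Casa flag once and calls OpenDoor.
; OpenDoor plays a timeline whose update sets the door to a fixed relative transform rather than interpolating.
; Once unlocked, a BP_TopDownChar overlapping the Box loads the Casa level.
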(event `Open Door`
  (`Timeline|Open Door Anim`
    (:`Update`
      (`SceneComponent.K2_SetRelativeLocationAndRotation` :`self` (`self.Door`) :`NewLocation` (77.0 69.0 0.0)))))

(event `Collect Item`
  (`/Engine/EditorBlueprintResources/StandardMacros.IncrementInt` (`self.currentItemCollected`)
    (:`  `
      (if (>= (`self.currentItemCollected`) (`self.maxItemsCollecatble`))
        (`/Engine/EditorBlueprintResources/StandardMacros.DoOnce` false
          (:`Completed`
            (set `self.casa` true)
            (`self.Open Door`)))))))

(event `self.Box.OnComponentBeginOverlap`
  (params (OverlappedComponent :type "PrimitiveComponent Object Reference") (OtherActor :type "Actor Object Reference") (OtherComp :type "PrimitiveComponent Object Reference") (OtherBodyIndex :type Integer) (bFromSweep :type Boolean) (SweepResult :type "HitResult Structure (by ref)"))
  (if (`self.casa`)
    (cast `/Game/Character/Sprites/BP_TopDownChar` OtherActor)
    (`GameplayStatics.OpenLevelBySoftObjectPtr` "/Game/Level/Casa.Casa")))

(fn `UserConstructionScript`)